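; BP_platform is a player-controlled platform that slides sideways and spawns BP_ball actors.
; The MoveRight axis moves it along Y in fixed per-tick steps by sign, without sweep or delta-time scaling.
; The Spawn_Ball event spawns a ball at the Arrow component's location.
; A Cube overlap with a BP_Bonus spawns another ball there through duplicated spawn logic, leaving the bonus untouched.
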(event OnComponentBeginOverlap(Cube)
  (params (OverlappedComponent :type Primitive%20Component%20Object%20Reference) (OtherActor :type Actor%20Object%20Reference) (OtherComp :type Primitive%20Component%20Object%20Reference) (OtherBodyIndex :type Integer) (bFromSweep :type Boolean) (SweepResult :type Hit%20Result%20Structure%20%28by%20ref%29))
  (Utilities|Casting|CastToBP_Bonus OtherActor)
  (Game|SpawnActorfromClass "/Game/MyLogic/task_1/BP_ball.BP_ball_C" (Math|Transform|MakeTransform (Transformation|GetWorldLocation (Variables|Default|GetArrow)) "0, 0, 0" "0.500000,1,1.000000") "Undefined" 0 0))

(event Custom|Spawn_Ball
  (Game|SpawnActorfromClass "/Game/MyLogic/task_1/BP_ball.BP_ball_C" (Math|Transform|MakeTransform (Transformation|GetWorldLocation (Variables|Default|GetArrow)) "0, 0, 0" "0.500000,1,1.000000") "Undefined" 0 0))

(event Input|AxisEvents|InputAxisMoveRight
  (params (AxisValue :type Float%20%28single-precision%29))
  (if (< AxisValue 0.0)
    (Transformation|AddActorWorldOffset "0,-50.000000, 0")))

(event Input|AxisEvents|InputAxisMoveRight
  (params (AxisValue :type Float%20%28single-precision%29))
  (if (> AxisValue 0.0)
    (Transformation|AddActorWorldOffset "0,50.000000, 0")))

(fn ConstructionScript)