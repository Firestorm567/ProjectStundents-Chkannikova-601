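; BP_Bonus is a moving bonus actor that randomly becomes one of two types, "long" or "ball", when play begins.
; The random pick sets Type and gives the Sphere a gold material for "long" or steel for "ball".
; Each tick moves it with sweep along its Location vector, scaled by Speed and delta time.
; The effect of each type is not applied in this Blueprint.
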(event EventBeginPlay
  (bind _sphere (Variables|Default|GetSphere))
  (if (Math|Random|RandomBool)
    (Variables|Default|Settype "long")
    (Rendering|Material|SetMaterial _sphere 0 "/Game/StarterContent/Materials/M_Metal_Gold.M_Metal_Gold")
    (else
      (Variables|Default|Settype "ball")
      (Rendering|Material|SetMaterial _sphere 0 "/Game/StarterContent/Materials/M_Metal_Steel.M_Metal_Steel"))))

(event EventTick
  (params (DeltaSeconds :type Float%20%28single-precision%29))
  (Transformation|AddActorWorldOffset (* (* (Variables|Default|Getlocation) (Variables|Default|Getspeed)) DeltaSeconds) true))

(fn ConstructionScript)